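; Pooled Gaster Blaster hazard that teleports to a random point in an arena box, turns toward the player and fires a Niagara beam near them.
; BlasterSpawn sequences blink effect, sound, animations and delays, stops aiming on firing, then BlasterDespawn hides the mesh and returns it to the BP_GasterBlasterPool location.
; Active toggles visibility, tick and a time-to-live timer calling ReturnToPool, whose SetInUSe function is empty.
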(event `self.ReceiveBeginPlay`
  (bind _outactors (`GameplayStatics.GetAllActorsOfClass` "/Game/_Content/_Characters/GasterBlaster/BP_GasterBlasterPool.BP_GasterBlasterPool_C"))
  (for _array_element _outactors
    _)
  (set `self.GasterBlasterPool` _array_element)
  (`ActorComponent.Deactivate` (`self.NS_BlasterShot`)))

(event `Active`
  (params (InUse :type Boolean))
  (set `self.InUse` InUse)
  (`self.SetActorHiddenInGame` (not InUse))
  (`self.SetActorTickEnabled` InUse)
  (`KismetSystemLibrary.K2_ClearAndInvalidateTimerHandle` (`self.timeToLiveTimer`))
  (if InUse
    (bind _returnvalue (`KismetSystemLibrary.K2_SetTimerDelegate` (delegate `ReturnToPool`) (`self.timeToLiveTime`)))
    (set `self.timeToLiveTimer` _returnvalue)))

(event `ReturnToPool`
  (`self.SetInUSe` (stale `Active` InUse)))

(event `self.ReceiveTick`
  (params (DeltaSeconds :type "Float (single-precision)"))
  (if (`self.IsAIming`)
    (`self.K2_SetActorRotation` (`KismetMathLibrary.FindLookAtRotation` (`self.K2_GetActorLocation`) (`self.K2_GetActorLocation` (`GameplayStatics.GetPlayerCharacter` 0))))))

(event `Blaster Spawn`
  (bind _returnvalue (`GameplayStatics.GetPlayerCharacter` 0))
  (bind _returnvalue_2 (`KismetMathLibrary.RandomPointInBoundingBox` (10.0 -1220.0 520.0) (650.0 2500.0 200.0)))
  (bind _ns_blastershot (`self.NS_BlasterShot`))
  (bind _randomlocation (`NavigationSystemV1.K2_GetRandomReachablePointInRadius` (+ (`self.K2_GetActorLocation` _returnvalue) (* (`self.GetActorForwardVector` _returnvalue) -25.0)) 50.0 null null))
  ; Activation/Deactivation
  (set `self.IsAIming` true)
  (`self.K2_SetActorLocation` _returnvalue_2 false true)
  (`GameplayStatics.PlaySoundAtLocation` "/Game/_Content/_Audio/SFX/SC_BlasterSpawn.SC_BlasterSpawn" _returnvalue_2 (struct) 1.0 1.0 0.0 null null null null)
  (`ActorComponent.Activate` (`self.NS_Blink_Fire`) true)
  (`KismetSystemLibrary.Delay` 0.5)
  (`SceneComponent.SetVisibility` (`self.GasterBlaster`) true false)
  (`KismetSystemLibrary.Delay` 2.0)
  (`SkeletalMeshComponent.PlayAnimation` (`self.GasterBlaster`) "/Game/_Content/_Characters/GasterBlaster/A_GasterBlaster_Blast.A_GasterBlaster_Blast" false)
  (`KismetSystemLibrary.Delay` 0.7)
  (if (not (== (`self.K2_GetActorLocation` (`self.GasterBlasterPool`)) (`self.K2_GetActorLocation`)))
    (`ActorComponent.Activate` _ns_blastershot true)
    (`NiagaraComponent.SetVariableVec3` _ns_blastershot "Beam End" (`KismetMathLibrary.MakeVector` (.x _randomlocation) (.y _randomlocation)))
    (if true
      (set `self.IsAIming` false)
      (`GameplayStatics.PlaySound2D` "/Game/_Content/_Audio/SFX/BlasterSound/BlasterBlast.BlasterBlast" 1.0 1.0 0.0 null null)
      (`KismetSystemLibrary.Delay` 2.0)
      (`SkeletalMeshComponent.PlayAnimation` (`self.GasterBlaster`) "/Game/_Content/_Characters/GasterBlaster/A_GasterBlaster_Idle.A_GasterBlaster_Idle" false)
      (`self.Blaster Despawn`))))

(event `Blaster Despawn`
  ; Activation/Deactivation
  (`ActorComponent.Activate` (`self.NS_Blink_Fire`) true)
  (`SceneComponent.SetVisibility` (`self.GasterBlaster`) false false)
  (`KismetSystemLibrary.Delay` 0.5)
  (`self.K2_SetActorLocation` (`self.K2_GetActorLocation` (`self.GasterBlasterPool`)) false true))

(fn `SetInUSe`
  (params (InUse1 :type Boolean)))

(fn `UserConstructionScript`)