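; BP_GasterBlasterPool is an object pool that fires Gaster Blaster attacks from pre-placed BP_GasterBlaster actors.
; On BeginPlay it gathers every blaster in the level and teleports them to its own location.
; Blast1 fires one shot and Blast2 fires two delayed pairs through BlasterShoot.
; BlasterShoot checks InUse and calls BlasterSpawn on random picks, re-rolled at each access, without retrying busy ones.
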(event `self.ReceiveBeginPlay`
  (bind _outactors (`GameplayStatics.GetAllActorsOfClass` "/Game/_Content/_Characters/GasterBlaster/BP_GasterBlaster.BP_GasterBlaster_C"))
  (bind _output_get (set `self.BlasterPool` _outactors))
  (for _array_element _output_get
    (`self.K2_TeleportTo` :`self` _array_element :`DestLocation` (`self.K2_GetActorLocation`))))

(event `Blast1`
  (`self.BlasterShoot`))

(event `Blast2`
  (`self.BlasterShoot`)
  (`self.BlasterShoot`)
  (`KismetSystemLibrary.Delay` 0.5)
  (`self.BlasterShoot`)
  (`self.BlasterShoot`))

(event `BlasterShoot`
  (bind _outitem (`KismetArrayLibrary.Array_Random` (`self.BlasterPool`)))
  (if (not (`/Game/_Content/_Characters/GasterBlaster/BP_GasterBlaster.InUse` _outitem))
    (set `/Game/_Content/_Characters/GasterBlaster/BP_GasterBlaster.InUse` true _outitem)
    (`/Game/_Content/_Characters/GasterBlaster/BP_GasterBlaster.Blaster Spawn` _outitem)))

(fn `UserConstructionScript`)