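; BP_BoneAttack_1 is a reusable bone attack hazard that parks at the BP_AttackCollector actor instead of being destroyed.
; On BeginPlay it finds the collector, caches actors tagged "StructureObstalce", and teleports to the collector.
; PlayerDetection overlap with the third-person character plays a damage sound and returns it there, without applying damage here.
; ObstacleDetection overlap with a cached obstacle also returns it; movement is not handled in this Blueprint.
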(event `self.ReceiveBeginPlay`
  (bind _outactors (`GameplayStatics.GetAllActorsOfClass` "/Game/_Content/_Characters/GasterBlaster/Bones/BP_AttackCollector.BP_AttackCollector_C"))
  (for _array_element _outactors
    (set `self.AttackCollector` _array_element)
    (bind _outactors_2 (`GameplayStatics.GetAllActorsWithTag` "StructureObstalce"))
    (set `self.StructureObstacles` _outactors_2)
    (`self.K2_SetActorLocation` (`self.K2_GetActorLocation` (`self.AttackCollector`)) false true)))

(event `self.PlayerDetection.OnComponentBeginOverlap`
  (params (OverlappedComponent :type "PrimitiveComponent Object Reference") (OtherActor :type "Actor Object Reference") (OtherComp :type "PrimitiveComponent Object Reference") (OtherBodyIndex :type Integer) (bFromSweep :type Boolean) (SweepResult :type "HitResult Structure (by ref)"))
  ; PlayerDetection
  (cast `/Game/ThirdPerson/Blueprints/BP_ThirdPersonCharacter` OtherActor)
  (`GameplayStatics.PlaySound2D` "/Game/_Content/_Audio/SFX/SC_DamageTaken.SC_DamageTaken" 1.0 1.0 0.0 null null)
  (`self.K2_SetActorLocation` (`self.K2_GetActorLocation` (`self.AttackCollector`)) false true))

(event `self.ObstacleDetection.OnComponentBeginOverlap`
  (params (OverlappedComponent :type "PrimitiveComponent Object Reference") (OtherActor :type "Actor Object Reference") (OtherComp :type "PrimitiveComponent Object Reference") (OtherBodyIndex :type Integer) (bFromSweep :type Boolean) (SweepResult :type "HitResult Structure (by ref)"))
  ; ObstacleDetection
  (for _array_element (`self.StructureObstacles`)
    (if (== OtherActor _array_element)
      (`self.K2_SetActorLocation` (`self.K2_GetActorLocation` (`self.AttackCollector`)) false true))))

(fn `UserConstructionScript`)