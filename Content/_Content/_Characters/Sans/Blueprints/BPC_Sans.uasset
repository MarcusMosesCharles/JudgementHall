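; Sans character that turns to face the player and dodges by teleporting between placed BP_Sans_TeleportPoints actors.
; BeginPlay caches the points, while Tick repeatedly sets a looping timer that eases yaw toward the player controller's location.
; Dodge fires a blink effect and rerolls random points until one has no player detected.
; The teleport then draws location and rotation from fresh random picks, so the destination can differ from the checked point.
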(event `self.ReceiveBeginPlay`
  (bind _outactors (`GameplayStatics.GetAllActorsOfClass` "/Game/_Content/_Characters/Sans/Blueprints/BP_Sans_TeleportPoints.BP_Sans_TeleportPoints_C"))
  (set `self.TeleportationPoints` _outactors))

(event `self.ReceiveTick`
  (params (DeltaSeconds :type "Float (single-precision)"))
  (`KismetSystemLibrary.K2_SetTimerDelegate` (delegate `Rotate`) 0.01 true))

(event `Rotate`
  (bind (_returnvalue_roll _returnvalue_pitch _returnvalue_yaw) (`KismetMathLibrary.BreakRotator` (`KismetMathLibrary.RInterpTo` (`self.K2_GetActorRotation`) (`KismetMathLibrary.FindLookAtRotation` (`self.K2_GetActorLocation`) (`self.K2_GetActorLocation` (`GameplayStatics.GetPlayerController` 0))) (`GameplayStatics.GetWorldDeltaSeconds`))))
  (`self.K2_SetActorRotation` (`KismetMathLibrary.MakeRotator` 0.0 0.0 _returnvalue_yaw)))

(fn `Dodge`
  (bind _outitem (`KismetArrayLibrary.Array_Random` (`self.TeleportationPoints`)))
  (`ActorComponent.Activate` (`self.NS_Blink_Fire`) false)
  (bind _asbp_sans_teleport_points (cast `/Game/_Content/_Characters/Sans/Blueprints/BP_Sans_TeleportPoints` _outitem :!label _label))
  (if (`/Game/_Content/_Characters/Sans/Blueprints/BP_Sans_TeleportPoints.PlayerDetected` _asbp_sans_teleport_points)
    (goto _label)
    (else
      (`self.K2_TeleportTo` (`self.K2_GetActorLocation` _outitem) (`self.K2_GetActorRotation` _outitem)))))

(fn `UserConstructionScript`)