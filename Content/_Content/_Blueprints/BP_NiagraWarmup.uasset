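; BP_NiagraWarmup is a Blueprint that briefly runs a set of Niagara effects at BeginPlay, apparently to warm them up before gameplay uses them.
; It activates six Niagara components covering knife slash, sparkles, blink fire, vampire dash and dust effects.
; After a short delay it deactivates all of them, with no other logic or construction script work.
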(event `self.ReceiveBeginPlay`
  (`ActorComponent.Activate` (`self.NS_KnifeSlash`) false)
  (`ActorComponent.Activate` (`self.NS_MainSparkle`) false)
  (`ActorComponent.Activate` (`self.NS_Sparkles`) false)
  (`ActorComponent.Activate` (`self.NS_Blink_Fire`) false)
  (`ActorComponent.Activate` (`self.NS_Dash_Vampire`) false)
  (`ActorComponent.Activate` (`self.NS_Dust`) false)
  (`KismetSystemLibrary.Delay` 0.2)
  (`ActorComponent.Deactivate` (`self.NS_KnifeSlash`))
  (`ActorComponent.Deactivate` (`self.NS_MainSparkle`))
  (`ActorComponent.Deactivate` (`self.NS_Sparkles`))
  (`ActorComponent.Deactivate` (`self.NS_Blink_Fire`))
  (`ActorComponent.Deactivate` (`self.NS_Dash_Vampire`))
  (`ActorComponent.Deactivate` (`self.NS_Dust`)))

(fn `UserConstructionScript`)