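; BP_GameMaster is a game manager that starts the Judgement Hall cutscene from a player interaction.
; It caches the third-person player character on BeginPlay.
; PlayerInteractionTrigger checks that the player is inside the first interaction volume, then creates and plays the LS_JudgementHall level sequence.
; It also hides the player and Enemy1 meshes, ducks the background sound and starts a camera fade, with no restore logic here.
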(event `self.ReceiveBeginPlay`
  (bind _asbp_third_person_character (cast `/Game/ThirdPerson/Blueprints/BP_ThirdPersonCharacter` (`GameplayStatics.GetPlayerPawn` 0)))
  (set `self.Player` _asbp_third_person_character))

(fn `Player Interaction Trigger`
  (if (`/Game/_Content/_Blueprints/Volumes/BP_FirstInteractionVolume.PlayerInBox` (`self.FirstInteractionVolume`))
    (bind _outactor (`LevelSequencePlayer.CreateLevelSequencePlayer` "/Game/_Content/_LevelSequencer/LS_JudgementHall.LS_JudgementHall"))
    (`MovieSceneSequencePlayer.Play` (`LevelSequenceActor.SequencePlayer` _outactor))
    (`SceneComponent.SetVisibility` (`Character.Mesh` (`self.Player`)) false false)
    (`SceneComponent.SetVisibility` (`Character.Mesh` (`self.Enemy1`)) false false)
    (`AudioComponent.AdjustVolume` (`AmbientSound.AudioComponent` (`self.BackgroundSound`)) 1.0 0.1 "Linear")
    (`PlayerCameraManager.StartCameraFade` :`self` (`GameplayStatics.GetPlayerCameraManager` 0) :`FromAlpha` 2.0 :`Duration` 1.0)))

(fn `UserConstructionScript`)